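; Moving platform Blueprint whose mesh material shows whether the platform is moving.
; On BeginPlay it sets the mesh to blue plastic when IsMoving is true, otherwise to a Phong material.
; An actor overlap passes the other actor to BeginOverlap, then reapplies the same material choice.
; The graph contains no movement logic, and Tick and the construction script are empty.
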(event EventBeginPlay
  (bind _meshcomponent (Variables|Default|GetMeshComponent))
  (if (Variables|Default|GetIsMoving)
    (Rendering|Material|SetMaterial _meshcomponent 0 "/Game/Materials/M_BluePlastic.M_BluePlastic")
    (else
      (Rendering|Material|SetMaterial _meshcomponent 0 "/Game/IceSpirit/phong1.phong1"))))

(event Collision|EventActorBeginOverlap
  (params (OtherActor :type Actor%20Object%20Reference))
  (bind _meshcomponent (Variables|Default|GetMeshComponent))
  (Class|PlatformMoving|BeginOverlap OtherActor)
  (if (Variables|Default|GetIsMoving)
    (Rendering|Material|SetMaterial _meshcomponent 0 "/Game/Materials/M_BluePlastic.M_BluePlastic")
    (else
      (Rendering|Material|SetMaterial _meshcomponent 0 "/Game/IceSpirit/phong1.phong1"))))

(event EventTick
  (params (DeltaSeconds :type Float%20%28single-precision%29)))

(fn ConstructionScript)