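; GM_FireAndIce, apparently the game mode, respawns the player's FireSpirit_Character after it is destroyed.
; On BeginPlay it casts the player character and binds to its OnDestroyed event.
; That handler waits briefly, spawns a new character at CharTransform, which is not assigned in these graphs, and has the first player controller possess it.
; It then calls Respawn to rebind the destroy event on the new character, so the cycle repeats.
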(event Custom|OnDestroyed_0
  (params (DestroyedActor :type Actor%20Object%20Reference))
  (Utilities|FlowControl|Delay 2.0)
  (bind _returnvalue (Game|SpawnActorfromClass "/Game/Blueprints/FireSpirit_Character.FireSpirit_Character_C" (Variables|Default|GetCharTransform) "Undefined" 0 0))
  (Pawn|Possess (Game|GetPlayerController 0) _returnvalue)
  (CallFunction|Respawn))

(event Custom|Respawn
  (bind _asfire_spirit_character (Utilities|Casting|CastToFireSpirit_Character (Game|GetPlayerCharacter 0)))
  (Game|BindEventtoOnDestroyed _asfire_spirit_character (delegate Custom|OnDestroyed_0)))

(event EventBeginPlay
  (bind _asfire_spirit_character (Utilities|Casting|CastToFireSpirit_Character (Game|GetPlayerCharacter 0)))
  (Game|BindEventtoOnDestroyed _asfire_spirit_character (delegate Custom|OnDestroyed_0)))

(event EventTick
  (params (DeltaSeconds :type Float%20%28single-precision%29)))

(fn ConstructionScript)