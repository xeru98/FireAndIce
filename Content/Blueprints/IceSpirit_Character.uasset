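; Playable Ice Spirit character for the Fire and Ice game mode, with mouse look scaled by the game mode's sensitivity settings.
; Tick drives movement; holding Space repeatedly jumps and ramps walk speed up to a cap, resetting it on release.
; Fire spawns an ice projectile at the muzzle.
; Cameras toggle on key 1 and auto-switch to first person when the main camera nears the capsule, with focal distance updated each tick.
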(event EventBeginPlay
  (bind _asgm_fire_and_ice (Utilities|Casting|CastToGM_FireAndIce (Game|GetGameMode)))
  (bind _output_get (Variables|Default|SetGM_Ref _asgm_fire_and_ice))
  (Variables|/Game/Blueprints/GM_FireAndIce.GM_FireAndIce_C|SetCharTransform _output_get (Transformation|GetActorTransform))
  (Input|SetInputModeGameOnly (Game|GetPlayerController 0)))

(event EventPossessed
  (params (NewController :type Controller%20Object%20Reference))
  (bind _asgm_fire_and_ice (Utilities|Casting|CastToGM_FireAndIce (Game|GetGameMode)))
  (bind _output_get (Variables|Default|SetGM_Ref _asgm_fire_and_ice))
  (Variables|/Game/Blueprints/GM_FireAndIce.GM_FireAndIce_C|SetCharTransform _output_get (Transformation|GetActorTransform))
  (Input|SetInputModeGameOnly (Game|GetPlayerController 0)))

(event EventTick
  (params (DeltaSeconds :type Float%20%28single-precision%29))
  (bind _charactermovement (Variables|Character|GetCharacterMovement))
  (Utilities|UpdateCameraFocus
    (:Out
      (Pawn|Input|AddMovementInput (Transformation|GetActorForwardVector) (Input|AxisValues|GetMoveForward) false)
      (Pawn|Input|AddMovementInput (Transformation|GetActorRightVector) (Input|AxisValues|GetMoveRight) false)
      (Utilities|FlowControl|Sequence
        (:then_0
          (if (Variables|Default|GetJump_1)
            (Character|Jump)
            (Variables|/Script/Engine.CharacterMovementComponent|SetMaxWalkSpeed _charactermovement (+ (Variables|/Script/Engine.CharacterMovementComponent|GetMaxWalkSpeed _charactermovement) 0.5))
            (else
              (Variables|/Script/Engine.CharacterMovementComponent|SetMaxWalkSpeed _charactermovement 2e+02))))
        (:then_2
          (Math|Integer|CompareInt (Math|Float|Truncate (Class|MovementComponent|GetMaxSpeed (Variables|Character|GetCharacterMovement))) 800
            (:>
              (Variables|Default|SetSpeedlimit true)
              (Variables|/Script/Engine.CharacterMovementComponent|SetMaxWalkSpeed _charactermovement 8e+02))
            (:<
              (Variables|Default|SetSpeedlimit false))))))))

(event Input|ActionEvents|InputActionFire
  (params (Key :type Key%20Structure))
  ;[1 1 1] Primary and Secondary Fire
  (:Pressed
    (Game|SpawnActorfromClass "/Game/Blueprints/Projectile_Ice.Projectile_Ice_C" (Transformation|GetWorldTransform (Variables|Default|GetMuzzle)) "AdjustIfPossibleButAlwaysSpawn" 0 0)))

(event Input|AxisEvents|InputAxisTurn
  (params (AxisValue :type Float%20%28single-precision%29))
  (Pawn|Input|AddControllerYawInput (* (Variables|/Game/Blueprints/GM_FireAndIce.GM_FireAndIce_C|GetSensitivityHorizontal (Variables|Default|GetGM_Ref)) AxisValue 1.0)))

(event Input|AxisEvents|InputAxisLookUp
  (params (AxisValue :type Float%20%28single-precision%29))
  (Pawn|Input|AddControllerPitchInput (* AxisValue (Variables|/Game/Blueprints/GM_FireAndIce.GM_FireAndIce_C|GetSensitivityVertical (Variables|Default|GetGM_Ref)) 1.0)))

(event Input|KeyboardEvents|SpaceBar
  (params (Key :type Key%20Structure))
  (:Pressed
    (Variables|Default|SetJump_1 true))
  (:Released
    (Variables|Default|SetJump_1 false)))

(event Input|KeyboardEvents|1
  (params (Key :type Key%20Structure))
  (bind _firstpersoncamera (Variables|Default|GetFirstPersonCamera))
  (bind _main_camera (Variables|Default|GetMain%20Camera))
  (:Pressed
    (Utilities|FlowControl|FlipFlop
      (:A
        (Components|Activation|SetActive _main_camera false false)
        (Components|Activation|SetActive _firstpersoncamera true false))
      (:B
        (Components|Activation|SetActive _main_camera true false)
        (Components|Activation|SetActive _firstpersoncamera false false)))))

(fn ConstructionScript)

(fn UpdateCameraFocalDistance
  (bind _main_camera (Variables|Default|GetMain%20Camera))
  (Variables|/Script/Engine.CameraComponent|SetPostProcessSettings _main_camera (Utilities|Struct|MakePostProcessSettings "DOFM_BokehDOF" (Math|Vector|VectorLength (- (Transformation|GetWorldLocation _main_camera) (Transformation|GetWorldLocation (Variables|Collision|GetCapsuleComponent self)))) 0.1 0.1 0.1)))