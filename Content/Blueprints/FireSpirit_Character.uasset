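; Player character for a fire-and-ice game that shoots fire and ice projectiles from its muzzle as primary and secondary fire.
; Tick applies movement input, calls Jump while Space is held to build walk speed up to a cap, resets it on release, and prints max speed.
; On possess or BeginPlay it stores its transform in GM_FireAndIce, whose sensitivity values scale look input, and sets game-only input for the player.
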(event EventBeginPlay
  (bind _returnvalue (Game|GetPlayerController 0))
  (bind _asgm_fire_and_ice (Utilities|Casting|CastToGM_FireAndIce (Game|GetGameMode)))
  (bind _output_get (Variables|Default|SetGM_Ref _asgm_fire_and_ice))
  (Variables|/Game/Blueprints/GM_FireAndIce.GM_FireAndIce_C|SetCharTransform _output_get (Transformation|GetActorTransform))
  (Utilities|Casting|CastToPC_FireandIce _returnvalue)
  (Utilities|Casting|CastToFireSpirit_Character (Game|Player|GetPlayerPawn 0))
  (Input|SetInputModeGameOnly _returnvalue))

(event EventPossessed
  (params (NewController :type Controller%20Object%20Reference))
  (bind _returnvalue (Game|GetPlayerController 0))
  (bind _asgm_fire_and_ice (Utilities|Casting|CastToGM_FireAndIce (Game|GetGameMode)))
  (bind _output_get (Variables|Default|SetGM_Ref _asgm_fire_and_ice))
  (Variables|/Game/Blueprints/GM_FireAndIce.GM_FireAndIce_C|SetCharTransform _output_get (Transformation|GetActorTransform))
  (Utilities|Casting|CastToPC_FireandIce _returnvalue)
  (Utilities|Casting|CastToFireSpirit_Character (Game|Player|GetPlayerPawn 0))
  (Input|SetInputModeGameOnly _returnvalue))

(event EventTick
  (params (DeltaSeconds :type Float%20%28single-precision%29))
  (bind _charactermovement (Variables|Character|GetCharacterMovement))
  (bind _charactermovement_2 (Variables|Character|GetCharacterMovement))
  (bind _returnvalue (Class|MovementComponent|GetMaxSpeed _charactermovement))
  (Pawn|Input|AddMovementInput (Transformation|GetActorForwardVector) (Input|AxisValues|GetMoveForward) false)
  (Pawn|Input|AddMovementInput (Transformation|GetActorRightVector) (Input|AxisValues|GetMoveRight) false)
  (Development|PrintString (Utilities|String|ToString(Float) _returnvalue) true true "(R=1.000000,G=0.053367,B=0.000000,A=1.000000)" 0.01)
  (Utilities|FlowControl|Sequence
    (:then_0
      (if (Variables|Default|GetJump_1)
        (Character|Jump)
        (Variables|/Script/Engine.CharacterMovementComponent|SetMaxWalkSpeed _charactermovement_2 (+ (Variables|/Script/Engine.CharacterMovementComponent|GetMaxWalkSpeed _charactermovement_2) 0.5))
        (else
          (Variables|/Script/Engine.CharacterMovementComponent|SetMaxWalkSpeed _charactermovement_2 2e+02))))
    (:then_2
      (Math|Integer|CompareInt (Math|Float|Truncate _returnvalue) 1500
        (:>
          (Variables|Default|SetSpeedlimit true)
          (Variables|/Script/Engine.CharacterMovementComponent|SetMaxWalkSpeed _charactermovement_2 1.5e+03))
        (:<
          (Variables|Default|SetSpeedlimit false))))))

(event Input|ActionEvents|InputActionFire
  (params (Key :type Key%20Structure))
  ;[1 1 1] Primary and Secondary Fire
  (:Pressed
    (Game|SpawnActorfromClass "/Game/Blueprints/Projectile_Fire.Projectile_Fire_C" (Transformation|GetWorldTransform (Variables|Default|GetMuzzle)) "AdjustIfPossibleButAlwaysSpawn" 0 0)))

(event Input|ActionEvents|InputActionSecondaryFire
  (params (Key :type Key%20Structure))
  ;[1 1 1] Primary and Secondary Fire
  (:Pressed
    (Game|SpawnActorfromClass "/Game/Blueprints/Projectile_Ice.Projectile_Ice_C" (Transformation|GetWorldTransform (Variables|Default|GetMuzzle)) "AdjustIfPossibleButAlwaysSpawn" 0 0)))

(event Input|AxisEvents|InputAxisTurn
  (params (AxisValue :type Float%20%28single-precision%29))
  (Pawn|Input|AddControllerYawInput (* (Variables|/Game/Blueprints/GM_FireAndIce.GM_FireAndIce_C|GetSensitivityHorizontal (Variables|Default|GetGM_Ref)) AxisValue)))

(event Input|AxisEvents|InputAxisLookUp
  (params (AxisValue :type Float%20%28single-precision%29))
  (Pawn|Input|AddControllerPitchInput (* AxisValue (Variables|/Game/Blueprints/GM_FireAndIce.GM_FireAndIce_C|GetSensitivityVertical (Variables|Default|GetGM_Ref)))))

(event Input|KeyboardEvents|SpaceBar
  (params (Key :type Key%20Structure))
  (:Pressed
    (Variables|Default|SetJump_1 true))
  (:Released
    (Variables|Default|SetJump_1 false)))

(fn ConstructionScript)