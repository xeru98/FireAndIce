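; Moving platform that projectiles switch on and off: a Projectile_Fire overlap starts it, a Projectile_Ice overlap stops it, and either projectile is destroyed.
; BeginPlay caches the world locations of the LocationA and LocationB markers, plus root-to-marker distances that the graph never reads.
; While moving, Tick sweeps the mesh toward the current target at MovementSpeed, flipping direction when within one frame's step of it.
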(event EventBeginPlay
  (Variables|Default|SetLocationAVector (Transformation|GetWorldLocation (Variables|Default|GetLocationA)))
  (Variables|Default|SetLocationBVector (Transformation|GetWorldLocation (Variables|Default|GetLocationB)))
  (bind _output_get (Variables|Default|SetRoot%20Location (Transformation|GetWorldLocation (Variables|Default|GetDefaultSceneRoot))))
  (Variables|Default|SetDistanceA (Utilities|VectorDistance _output_get (Variables|Default|GetLocationAVector)))
  (Variables|Default|SetDistanceB (Utilities|VectorDistance _output_get (Variables|Default|GetLocationBVector))))

(event Collision|EventActorBeginOverlap
  (params (OtherActor :type Actor%20Object%20Reference))
  (if (Actor|ActorHasTag OtherActor "Projectile_Fire")
    (Variables|Movement|SetIsMoving true)
    (Actor|DestroyActor OtherActor :!label _label)
    (elif (Actor|ActorHasTag OtherActor "Projectile_Ice")
      (Variables|Movement|SetIsMoving false)
      (goto _label))))

(event EventTick
  (params (DeltaSeconds :type Float%20%28single-precision%29))
  (bind _staticmesh (Variables|Default|GetStaticMesh))
  (bind _returnvalue (Transformation|GetWorldLocation _staticmesh))
  (if (Variables|Movement|GetIsMoving)
    (Variables|Default|SetDeltaMovement (* DeltaSeconds (Variables|Movement|GetMovementSpeed)))
    (Variables|Default|SetMeshLocation (Transformation|GetWorldLocation (Variables|Default|GetStaticMesh)))
    (if (Variables|Movement|GetTowardsA)
      (Variables|Default|SetDirectionVector (- (Variables|Default|GetLocationAVector) (Variables|Default|GetMeshLocation)))
      (else
        (Variables|Default|SetDirectionVector (- (Variables|Default|GetLocationBVector) (Variables|Default|GetMeshLocation)))))
    (Transformation|SetWorldLocation (Variables|Default|GetStaticMesh) (+ (* (Math|Vector|Normalize (Variables|Default|GetDirectionVector)) (Variables|Default|GetDeltaMovement)) (Variables|Default|GetMeshLocation)) true false)
    (if (Variables|Movement|GetTowardsA)
      (if (Math|Vector|Equal(Vector) _returnvalue (Variables|Default|GetLocationAVector) (Variables|Default|GetDeltaMovement))
        (Variables|Movement|SetTowardsA (not (Variables|Movement|GetTowardsA)) :!label _label))
      (elif (Math|Vector|Equal(Vector) _returnvalue (Variables|Default|GetLocationBVector) (Variables|Default|GetDeltaMovement))
        (goto _label)))))

(fn ConstructionScript)